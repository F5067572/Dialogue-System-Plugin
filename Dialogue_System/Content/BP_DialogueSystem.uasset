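; Interactable dialogue actor that plays a two-sided conversation in a W_DialogueWIdget while player movement is disabled.
; A short interaction starts it, stepping through parallel arrays of lines, names, sides and images.
; Delay loops type each line letter by letter into its side's text box, then auto-advance after a pause.
; Holding left mouse, polled on Tick, speeds up typing; the last line removes the widget and restores walking.
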(event `Next`
  ;[0 0.15 0.009951 0.5] Do Next: End/Restart
  (if (== (+ (`self.Array Index`) 1) (`KismetArrayLibrary.Array_Length` (`self.Dialogue`)))
    ;;[0.000315 0.08979 0.15 0.5] End
    (`Widget.RemoveFromParent` (`self.WidgetRef`))
    (`CharacterMovementComponent.SetMovementMode` (`Character.CharacterMovement` (`GameplayStatics.GetPlayerCharacter` 0)) "MOVE_Walking" 0)
    (`KismetSystemLibrary.Delay` 1.0)
    (set `self.DoNext?` false)
    (set `self.Going?` false)
    (else
      ;;[0.000315 0.08979 0.15 0.5] Restart
      (set `self.DoNext?` false)
      (`self.Restart`))))

(event `self.ReceiveTick`
  (params (DeltaSeconds :type "Float (single-precision)"))
  ;[0.0999 0.004391 0.004025] Speed Up/Down
  (`self.Switch Speed`))

(event `Restart`
  (bind _widgetref (`self.WidgetRef`))
  (bind _position_in_dialogue (`self.Position in dialogue`))
  (bind _widgetref_2 (`self.WidgetRef`))
  (bind _position_in_dialogue_2 (`self.Position in dialogue`))
  (bind _output (`|GetArrayItem` (`self.Dialogue`) (`self.Array Index`)))
  (bind _output_2 (`|GetArrayItem` (`self.CharacterImage`) (`self.Array Index`)))
  (bind _output_3 (`|GetArrayItem` (`self.Dialogue`) (`self.Array Index`)))
  (bind _output_4 (`|GetArrayItem` (`self.CharacterImage`) (`self.Array Index`)))
  (bind _characterside1 (`/Dialogue_System/W_DialogueWIdget.CharacterSide1` _widgetref_2))
  (bind _characterside2 (`/Dialogue_System/W_DialogueWIdget.CharacterSide2` _widgetref))
  ;[0.000315 0.08979 0.15 0.5] Doing Next dialogue in array
  (`/Engine/EditorBlueprintResources/StandardMacros.IncrementInt` (`self.Array Index`)
    (:`  `
      (if (not (`self.DoNext?`)) :!label _label
        (set `self.DoNext?` true)
        (if (== (`|GetArrayItem` (`self.Side`) (`self.Array Index`)) 1)
          ;[0 0.15 0.009951 0.5] Displaying Text - Both sides are the same with some variables changed
          ;;[0.000315 0.08979 0.15 0.5] Side 1 Text
          (`/Dialogue_System/W_DialogueWIdget.EnableSide1` (`self.WidgetRef`))
          (set `TextBlock.Text` (`KismetTextLibrary.Conv_StringToText` (`|GetArrayItem` (`self.Names`) (`self.Array Index`))) (`/Dialogue_System/W_DialogueWIdget.Name1` _widgetref_2))
          (`/Engine/EditorBlueprintResources/StandardMacros.IsValid` _output_2
            (:`Is Valid`
              (set `Image.Brush` (`Image.Brush` _characterside1) _output_2))
            (:`Is Not Valid`
              (`Widget.SetVisibility` _characterside1 "Hidden")))
          (set `self.dialoguestring` "")
          (set `self.Position in dialogue` 0)
          (set `self.Letters` (`KismetStringLibrary.GetCharacterArrayFromString` _output))
          (`self.Dialogue Typing for side 1` _position_in_dialogue_2 :!label _label_2)
          (`KismetSystemLibrary.Delay` (`self.Duration`))
          (if (< _position_in_dialogue_2 (`KismetStringLibrary.Len` _output))
            (`/Engine/EditorBlueprintResources/StandardMacros.IncrementInt` (`self.Position in dialogue`)
              (:`  `
                (goto _label_2)))
            (else
              (`KismetSystemLibrary.Delay` 2.0)
              (`self.Next`)))
          (else
            ;;[0.000315 0.08979 0.15 0.5] Side 2 Text
            (`/Dialogue_System/W_DialogueWIdget.EnableSide2` (`self.WidgetRef`))
            (set `TextBlock.Text` (`KismetTextLibrary.Conv_StringToText` (`|GetArrayItem` (`self.Names`) (`self.Array Index`))) (`/Dialogue_System/W_DialogueWIdget.Name2` _widgetref))
            (`/Engine/EditorBlueprintResources/StandardMacros.IsValid` _output_4
              (:`Is Valid`
                (set `Image.Brush` (`Image.Brush` _characterside2) _output_4))
              (:`Is Not Valid`
                (`Widget.SetVisibility` _characterside2 "Hidden")))
            (set `self.dialoguestring` "")
            (set `self.Position in dialogue` 0)
            (set `self.Letters` (`KismetStringLibrary.GetCharacterArrayFromString` _output_3))
            (`self.Dialogue Typing for side 2` _position_in_dialogue :!label _label_3)
            (`KismetSystemLibrary.Delay` (`self.Duration`))
            (if (< _position_in_dialogue (`KismetStringLibrary.Len` _output_3))
              (`/Engine/EditorBlueprintResources/StandardMacros.IncrementInt` (`self.Position in dialogue`)
                (:`  `
                  (goto _label_3)))
              (else
                (`KismetSystemLibrary.Delay` 2.0)
                (`self.Next`)))))))))

(event `self.InteractionComponent.OnShortInteraction`
  (params (Instigator :type "Actor Object Reference"))
  ;[0.0999 0.004391 0.004025] Start
  (if (not (`self.Going?`))
    (`CharacterMovementComponent.DisableMovement` (`Character.CharacterMovement` (`GameplayStatics.GetPlayerCharacter` 0)))
    (set `self.Going?` true)
    ;[0 1 0.6176 0.5] Creating Widget
    (bind _returnvalue (`|CreateWidget` "/Dialogue_System/W_DialogueWIdget.W_DialogueWIdget_C"))
    (bind _output_get (set `self.WidgetRef` _returnvalue))
    (`UserWidget.AddToViewport` _output_get 0)
    ;[0.000315 0.08979 0.15 0.5] Doing Next dialogue in array
    (set `self.Array Index` 0)
    (goto _label)))

(fn `Dialogue Typing for side 1`
  (params (Position :type Integer))
  (bind _output_get (set `self.dialoguestring` (`KismetStringLibrary.Concat_StrStr` (`self.dialoguestring`) (`|GetArrayItem` (`self.Letters`) Position))))
  (set `TextBlock.Text` (`KismetTextLibrary.Conv_StringToText` _output_get) (`/Dialogue_System/W_DialogueWIdget.DialougeTextBox1` (`self.WidgetRef`))))

(fn `Dialogue Typing for side 2`
  (params (Position :type Integer))
  (bind _output_get (set `self.dialoguestring` (`KismetStringLibrary.Concat_StrStr` (`self.dialoguestring`) (`|GetArrayItem` (`self.Letters`) Position))))
  (set `TextBlock.Text` (`KismetTextLibrary.Conv_StringToText` _output_get) (`/Dialogue_System/W_DialogueWIdget.DialougeTextBox2` (`self.WidgetRef`))))

(fn `Switch Speed`
  (bind _returnvalue (< (`self.Position in dialogue`) (`KismetStringLibrary.Len` (`|GetArrayItem` (`self.Dialogue`) (`self.Array Index`)))))
  (if (and (`self.Going?`) (`PlayerController.IsInputKeyDown` (`GameplayStatics.GetPlayerController` 0) "LeftMouseButton"))
    ; Checks to see if the speed is already doubled or not, then doubles or halfs it
    (if (and _returnvalue (not (`self.Skip`)))
      (set `self.Duration` (/ (`self.Duration`) 10.0))
      (set `self.Skip` true))
    (elif (and _returnvalue (`self.Skip`))
      (set `self.Duration` (* (`self.Duration`) 10.0))
      (set `self.Skip` false))))

(fn `UserConstructionScript`)